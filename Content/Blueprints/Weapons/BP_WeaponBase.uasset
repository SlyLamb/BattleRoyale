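; Base weapon Blueprint that tracks magazine and spare ammo for an owning BR_Character.
; BeginPlay, GiveAmmo and OnFired change state only on the authority, with GiveAmmo topping up the magazine before sending any remainder to capped spare ammo.
; Firing an empty-leaving shot triggers Reload, which flags the character as reloading, waits a fixed delay, then sets the magazine from spare ammo.
; HasAmmo reports whether the magazine holds rounds.
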(event `self.ReceiveBeginPlay`
  ;[1 1 1] Set up ammo amounts and owning player
  (`/Engine/EditorBlueprintResources/ActorMacros.Switch Has Authority`
    (:`Authority`
      (set `self.CurrentAmmo` (`self.MagSize`))
      (set `self.CurrentSpareAmmo` (`self.StartingSpareAmmo`))
      (bind _asbr_character (cast `/Game/BRGame/Blueprints/BR_Character` (`self.GetOwner`)))
      (set `self.OwningCharacter` _asbr_character))))

(event `Give Ammo`
  (params (`Ammo To Give` :type Integer))
  (bind _currentammo (`self.CurrentAmmo`))
  (bind _returnvalue (`KismetMathLibrary.Min` `Ammo To Give` (- (`self.MagSize`) _currentammo)))
  (bind _returnvalue_2 (- `Ammo To Give` _returnvalue))
  ;[1 1 1] Event to give ammo to weapon when needed
  (`/Engine/EditorBlueprintResources/ActorMacros.Switch Has Authority`
    (:`Authority`
      (set `self.CurrentAmmo` (+ _returnvalue _currentammo))
      (if (> _returnvalue_2 0)
        (set `self.CurrentSpareAmmo` (+ (`self.CurrentSpareAmmo`) (`KismetMathLibrary.Min` _returnvalue_2 (- (`self.MaxSpareAmmo`) (`self.CurrentSpareAmmo`)))))))))

(event `On Fired`
  (bind _currentammo (`self.CurrentAmmo`))
  ;[1 1 1] Fire and call reload
  (`/Engine/EditorBlueprintResources/ActorMacros.Switch Has Authority`
    (:`Authority`
      (`/Engine/EditorBlueprintResources/StandardMacros.DecrementInt` _currentammo
        (:`  `
          (if (<= _currentammo 0)
            (`self.Reload`)))))))

(event `Reload`
  (bind _returnvalue (`KismetMathLibrary.Min` (`self.CurrentSpareAmmo`) (`self.MagSize`)))
  ;[1 1 1] Reload
  (set `/Game/BRGame/Blueprints/BR_Character.IsReloading` true (`self.OwningCharacter`))
  (`KismetSystemLibrary.Delay` 2.2)
  (set `self.CurrentAmmo` _returnvalue)
  (set `self.CurrentSpareAmmo` (`KismetMathLibrary.Max` (- (`self.CurrentSpareAmmo`) _returnvalue)))
  (set `/Game/BRGame/Blueprints/BR_Character.IsReloading` false (`self.OwningCharacter`)))

(fn `HasAmmo`
  (returns (`Return Value` :type Boolean))
  (return (> (`self.CurrentAmmo`) 0)))

(fn `UserConstructionScript`)